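; Gas pickup actor that lets an overlapping ThirdPersonCharacter collect gas with the Interact input.
; Box begin overlap caches the character and enables input from player controller 0, and end overlap by any such character disables it.
; On Interact, it calls PickupGasOnServer on the cached character, then DestroyGasOnServer after a half-second delay, leaving both pickup and destruction to the character.
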(event OnComponentBeginOverlap(Box)
  (params (OverlappedComponent :type Primitive%20Component%20Object%20Reference) (OtherActor :type Actor%20Object%20Reference) (OtherComp :type Primitive%20Component%20Object%20Reference) (OtherBodyIndex :type Integer) (bFromSweep :type Boolean) (SweepResult :type Hit%20Result%20Structure%20%28by%20ref%29))
  (bind _asthird_person_character (Utilities|Casting|CastToThirdPersonCharacter OtherActor))
  (Variables|Default|SetAs%20Third%20Person%20Character _asthird_person_character)
  (Input|EnableInput (Game|GetPlayerController 0)))

(event OnComponentEndOverlap(Box)
  (params (OverlappedComponent :type Primitive%20Component%20Object%20Reference) (OtherActor :type Actor%20Object%20Reference) (OtherComp :type Primitive%20Component%20Object%20Reference) (OtherBodyIndex :type Integer))
  (Utilities|Casting|CastToThirdPersonCharacter OtherActor)
  (Input|DisableInput (Game|GetPlayerController 0)))

(event Input|ActionEvents|InputActionInteract
  (params (Key :type Key%20Structure :default "None"))
  (bind _as_third_person_character (Variables|Default|GetAs%20Third%20Person%20Character))
  (:Pressed
    (Default|PickupGasonServer _as_third_person_character true)
    (Utilities|FlowControl|Delay 0.5)
    (Default|DestroyGasonServer _as_third_person_character)))

(fn ConstructionScript)